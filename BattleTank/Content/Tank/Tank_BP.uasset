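; Tank Blueprint that sets up the barrel reference and handles player aim input.
; On BeginPlay it passes the Barrel component to SetBarrelReference.
; AimAzimuth yaws the SpringGimbal and AimElevation pitches the SpringArm, separating the two rotation axes across components.
; Both inputs scale by world delta time and a fixed rate for frame-rate-independent rotation.
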(event EventBeginPlay)

(event Collision|EventActorBeginOverlap
  (params (OtherActor :type Actor%20Object%20Reference)))

(event EventTick
  (params (DeltaSeconds :type Float%20%28single-precision%29)))

(event EventBeginPlay
  (Class|Tank|SetBarrelReference (Variables|Default|GetBarrel)))

(event Input|AxisEvents|InputAxisAimElevation
  (params (AxisValue :type Float%20%28single-precision%29))
  (Transformation|AddLocalRotation (Variables|Default|GetSpringArm) (Math|Rotator|MakeRotator 0.0 (* AxisValue (Utilities|Time|GetWorldDeltaSeconds) 6e+01) 0.0) false false))

(event Input|AxisEvents|InputAxisAimAzimuth
  (params (AxisValue :type Float%20%28single-precision%29))
  (Transformation|AddLocalRotation (Variables|Default|GetSpring%20Gimbal) (Math|Rotator|MakeRotator 0.0 0.0 (* AxisValue (Utilities|Time|GetWorldDeltaSeconds) 6e+01)) false false))

(fn ConstructionScript)